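; BP_Volume is a level-exit volume meant to complete the level when the player overlaps it with no BP_crystal actors left.
; Completion finds the current level in the LevelNames array, then opens the next entry or quits the game on the last.
; AnyCrystalRemaining tests the crystal count with >= 0, so it always returns true and completion never fires as written.
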(event EventBeginPlay)

(event Collision|EventActorBeginOverlap
  (params (OtherActor :type Actor%20Object%20Reference))
  (Utilities|IsPlayer OtherActor
    (:IsPlayer
      (if (not (CallFunction|AnyCrystalRemaining))
        (LevelManagement|CompleteLevel)))))

(event EventTick
  (params (DeltaSeconds :type Float%20%28single-precision%29)))

(fn ConstructionScript)

(fn AnyCrystalRemaining
  (bind _outactors (Actor|GetAllActorsOfClass "/Game/Blueprints/Actors/Collectibles/BP_crystal.BP_crystal_C"))
  (return (>= (Utilities|Array|Length _outactors) 0)))

(fn CompleteLevel
  (if (LevelManagement|IsFinalLevel)
    (Game|QuitGame 0 "Quit")
    (else
      (LevelManagement|LoadLevel))))

(fn GetCurrentLevelIndex
  (bind _returnvalue (Game|GetCurrentLevelName true))
  (return (Utilities|Array|FindItem (Variables|Default|GetLevel%20Names) (Utilities|String|StringToName _returnvalue))))

(fn IsFinalLevel
  (return (== (Utilities|Array|LastIndex (Variables|Default|GetLevel%20Names)) (LevelManagement|GetCurrentLevelIndex))))

(fn LoadLevel
  (Game|OpenLevel(byName) (LevelManagement|GetNextLevelName)))

(fn GetNextLevelName
  (return (Utilities|Array|Get(acopy) (Variables|Default|GetLevel%20Names) (+ (LevelManagement|GetCurrentLevelIndex) 1))))