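; BP_crystal is a collectible crystal actor that flies into the player on touch and then disappears.
; Overlap with the player pawn stores the crystal's current location and plays a timeline.
; Each update lerps the crystal from that stored point toward the pawn's live location using the timeline's alpha, so it homes in on a moving player.
; The actor destroys itself when the timeline finishes, with no reward logic.
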(event Collision|EventActorBeginOverlap
  (params (OtherActor :type Actor%20Object%20Reference))
  (if (== OtherActor (Game|Player|GetPlayerPawn 0))
    (Variables|Default|SetLERP%20Start%20Location (Transformation|GetActorLocation))
    (bind _alpha_smooth_change (Timeline|Timeline_0 Play)
      (:Update
        (Transformation|SetActorLocation (Math|Vector|Lerp(Vector) (Variables|Default|GetLERP%20Start%20Location) (Transformation|GetActorLocation (Game|Player|GetPlayerPawn 0)) _alpha_smooth_change) false false))
      (:Finished
        (Actor|DestroyActor)))))

(fn ConstructionScript)