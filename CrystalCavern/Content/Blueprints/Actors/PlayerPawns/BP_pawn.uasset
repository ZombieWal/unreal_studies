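; BP_pawn is a player pawn that moves a physics Ball by rolling it with torque.
; The Forward/Backward and Left/Right axis inputs apply torque around Y and X, scaled by TorqueStrength and applied as acceleration change so mass is ignored.
; BeginPlay starts a brief camera fade in from a near-black blue.
; Taking damage only prints a debug message, with no health logic.
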(event EventBeginPlay
  (CameraFades|StartCameraFade (Game|GetPlayerCameraManager 0) 1.0 0.0 1.0 "(R=0.011765,G=0.011765,B=0.058824,A=1.000000)" false false))

(event Collision|EventActorBeginOverlap
  (params (OtherActor :type Actor%20Object%20Reference)))

(event EventTick
  (params (DeltaSeconds :type Float%20%28single-precision%29)))

(event Game|Damage|EventAnyDamage
  (params (Damage :type Float%20%28single-precision%29) (DamageType :type Damage%20Type%20Object%20Reference) (InstigatedBy :type Controller%20Object%20Reference) (DamageCauser :type Actor%20Object%20Reference))
  (Development|PrintString "Emotional damage"))

(event Input|AxisEvents|InputAxisForward/Backward
  (params (AxisValue :type Float%20%28single-precision%29))
  (Class|PrimitiveComponent|AddTorqueinRadians (Variables|Default|GetBall) (Math|Vector|MakeVector 0.0 (* AxisValue (Variables|Default|GetTorqueStrength)) 0.0) "None" true))

(event Input|AxisEvents|InputAxisLeft/Right
  (params (AxisValue :type Float%20%28single-precision%29))
  (Class|PrimitiveComponent|AddTorqueinRadians (Variables|Default|GetBall) (Math|Vector|MakeVector (* AxisValue (Variables|Default|GetTorqueStrength)) 0.0 0.0) "None" true))

(fn ConstructionScript)