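; BP_Cannon is an actor that fires projectiles automatically and repeatedly from BeginPlay.
; After each FireRate delay, it spawns a BP_Projectile at the ProjectileBallSpawn component's location and rotation, scaled by ScaleBall.
; A timeline then animates the Cannon component along its relative Y axis to move the barrel.
; The timeline's event track loops back to the delay, so the barrel animation drives the next shot.
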(event EventBeginPlay
  (Utilities|FlowControl|Delay (Variables|Default|GetFireRate) :!label _label)
  (CallFunction|SpawnProjectile)
  (bind _barrel_location (Timeline|Barrel_Movement_Timeline PlayFromStart)
    (:Update
      (CallFunction|MoveCannonBarrel _barrel_location))
    (:Cannon%20FIred
      (goto _label))))

(event Collision|EventActorBeginOverlap
  (params (OtherActor :type Actor%20Object%20Reference)))

(event EventTick
  (params (DeltaSeconds :type Float%20%28single-precision%29)))

(fn ConstructionScript)

(fn SpawnProjectile
  (bind _projectileballspawn (Variables|Default|GetProjectileBallSpawn))
  (Game|SpawnActorfromClass "/Game/Blueprints/Actors/Volumes/BP_Projectile.BP_Projectile_C" (Math|Transform|MakeTransform (Transformation|GetWorldLocation _projectileballspawn) (Transformation|GetWorldRotation _projectileballspawn) (Math|Conversions|ToVector(Float) (Variables|Default|GetScaleBall))) "Undefined" 0 0))

(fn MoveCannonBarrel
  (params (Cannon%20Barrel%20Y%20Location :type Float%20%28single-precision%29))
  (Transformation|SetRelativeLocation (Variables|Default|GetCannon) (Math|Vector|MakeVector 0.0 Cannon%20Barrel%20Y%20Location 0.0) false false))